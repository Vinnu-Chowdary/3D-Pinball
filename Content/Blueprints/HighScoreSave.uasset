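; High score save Blueprint that keeps a leaderboard of the top three score entries in SaveStruct.
; AddHighScore appends a new entry, sorts the array from highest to lowest, then trims it to at most three.
; SortSaveData is a selection sort that repeatedly moves the DetermineHighestScore result into TempSaveStruct, then copies that back.
; DetermineLowestScoreValue returns the lowest entry and its index but is not called here.
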(fn `AddHighScore`
  (params (NewScore :type "/Game/Blueprints/HighScoreStruct Structure"))
  (bind _save_struct (`self.Save Struct`))
  (`KismetArrayLibrary.Array_Add` (`self.Save Struct`) NewScore)
  (`self.SortSaveData`)
  (`KismetArrayLibrary.Array_Resize` _save_struct (`KismetMathLibrary.Min` 3 (`KismetArrayLibrary.Array_Length` _save_struct))))

(fn `DetermineHighestScore`
  (returns (HighestScoreStruct :type "/Game/Blueprints/HighScoreStruct Structure") (HighestScoreIndex :type Integer))
  (locals (HighestScore :type "Float (double-precision)") (Highestindex :type Integer))
  (bind _highestindex (`local.Highestindex`))
  (for (_array_element _array_index) (`self.Save Struct`)
    (if (== _array_index 0)
      (set `local.HighestScore` (`.Score_5_BF8D1ED74AC7583B0A439B8B1F711423` (break `/Game/Blueprints/HighScoreStruct` _array_element)))
      (set `local.Highestindex` _array_index)
      (elif (> (`.Score_5_BF8D1ED74AC7583B0A439B8B1F711423` (break `/Game/Blueprints/HighScoreStruct` _array_element)) (`local.HighestScore`))
        (set `local.HighestScore` (`.Score_5_BF8D1ED74AC7583B0A439B8B1F711423` (break `/Game/Blueprints/HighScoreStruct` _array_element)))
        (set `local.Highestindex` _array_index))))
  (return (`|GetArrayItem` (`self.Save Struct`) _highestindex) _highestindex))

(fn `DetermineLowestScoreValue`
  (returns (LowestScoreStruct :type "/Game/Blueprints/HighScoreStruct Structure") (LowestScoreIndex :type Integer))
  (locals (LowestScore :type "Float (double-precision)") (Lowestindex :type Integer))
  (bind _lowestindex (`local.Lowestindex`))
  (for (_array_element _array_index) (`self.Save Struct`)
    (if (== _array_index 0)
      (set `local.LowestScore` (`.Score_5_BF8D1ED74AC7583B0A439B8B1F711423` (break `/Game/Blueprints/HighScoreStruct` _array_element)))
      (set `local.Lowestindex` _array_index)
      (elif (< (`.Score_5_BF8D1ED74AC7583B0A439B8B1F711423` (break `/Game/Blueprints/HighScoreStruct` _array_element)) (`local.LowestScore`))
        (set `local.LowestScore` (`.Score_5_BF8D1ED74AC7583B0A439B8B1F711423` (break `/Game/Blueprints/HighScoreStruct` _array_element)))
        (set `local.Lowestindex` _array_index))))
  (return (`|GetArrayItem` (`self.Save Struct`) _lowestindex) _lowestindex))

(fn `SortSaveData`
  (while (> (`KismetArrayLibrary.Array_Length` (`self.Save Struct`)) 0)
    (bind (_highestscorestruct _highestscoreindex) (`self.DetermineHighestScore`))
    (`KismetArrayLibrary.Array_Add` (`self.TempSaveStruct`) _highestscorestruct)
    (`KismetArrayLibrary.Array_Remove` (`self.Save Struct`) _highestscoreindex))
  (set `self.Save Struct` (`self.TempSaveStruct`)))